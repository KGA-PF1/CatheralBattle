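; BP_Boss_Sevarog is the Sevarog boss Blueprint that runs the death and game-ending sequence.
; Tick watches Hp and, once it drops to zero, removes all widgets a single time and plays the Boss_Death level sequence.
; When that sequence finishes, the Ending sequence plays, and its completion creates and shows the UI_ENDING widget.
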(event Custom|Ending
  (bind _returnvalue (Sequencer|Player|CreateLevelSequencePlayer "/Game/TeamShare/TeamShare_CSW/CutScene/Ending.Ending"))
  (Sequencer|Player|Play _returnvalue :!class /Script/MovieScene.MovieSceneSequencePlayer)
  (EventDispatchers|AssignOnFinished _returnvalue (delegate Custom|CustomEvent)))

(event Custom|CustomEvent
  (bind _returnvalue (UserInterface|CreateWidget "/Game/TeamShare/TeamShare_KSW/UI_ENDING.UI_ENDING_C"))
  (bind _output_get (Variables|Default|SetUIEnding _returnvalue))
  (UserInterface|Viewport|AddtoViewport _output_get 0))

(event EventBeginPlay)

(event Collision|EventActorBeginOverlap
  (params (OtherActor :type Actor%20Object%20Reference)))

(event EventTick
  (params (DeltaSeconds :type Float%20%28single-precision%29))
  (if (<= (Variables|Default|GetHp) 0.0)
    (Utilities|FlowControl|DoOnce false
      (:Completed
        (Viewport|RemoveAllWidgets)
        (bind _returnvalue (Sequencer|Player|CreateLevelSequencePlayer "/Game/TeamShare/TeamShare_CSW/CutScene/Boss_Death.Boss_Death"))
        (Sequencer|Player|Play _returnvalue :!class /Script/MovieScene.MovieSceneSequencePlayer)
        (EventDispatchers|BindEventtoOnFinished _returnvalue (delegate Custom|Ending))))))

(fn ConstructionScript)