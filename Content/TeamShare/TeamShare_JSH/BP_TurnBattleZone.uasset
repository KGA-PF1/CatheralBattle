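; BP_TurnBattleZone is a trigger volume that starts a turn-based boss battle the first time the player character overlaps its box.
; On overlap it latches a one-shot flag, uses AutoFind to grab the first BattleManager (if unset) and Boss_Sevarog in the level, then waits a test cutscene delay.
; When the timer fires, it validates manager, boss and player, then initializes and starts the battle, with debug prints for validity and failures.
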(event OnComponentBeginOverlap(Box)
  (params (OverlappedComponent :type Primitive%20Component%20Object%20Reference) (OtherActor :type Actor%20Object%20Reference) (OtherComp :type Primitive%20Component%20Object%20Reference) (OtherBodyIndex :type Integer) (bFromSweep :type Boolean) (SweepResult :type Hit%20Result%20Structure%20%28by%20ref%29))
  (if (not (Variables|Default|GetbTriggered))
    (Utilities|Casting|CastToBP_PlayerCharacter OtherActor)
    (Variables|Default|SetbTriggered true)
    (CallFunction|AutoFind)
    (Utilities|Time|SetTimerbyEvent (delegate Custom|BeginTurnBattle) (Variables|Default|GetTestCutsceneSec))))

(event Custom|BeginTurnBattle
  (bind _battlemanager (Variables|Default|GetBattleManager))
  (bind _boss (Variables|Default|GetBoss))
  (bind _returnvalue (Utilities|IsValid _battlemanager))
  (bind _returnvalue_2 (Utilities|IsValid _boss))
  (bind _asbp_player_character (Utilities|Casting|CastToBP_PlayerCharacter (Game|Player|GetPlayerPawn 0))
    (:then
      (Variables|Default|SetPlayer _asbp_player_character)
      (Development|PrintString (Utilities|String|ToString(Boolean) _returnvalue) true true "(R=1.000000,G=0.000000,B=0.096778,A=1.000000)")
      (Development|PrintString (Utilities|String|ToString(Boolean) _returnvalue_2) true true "(R=1.000000,G=0.322722,B=0.172612,A=1.000000)")
      (Development|PrintString (Utilities|String|ToString(Boolean) (Utilities|IsValid (Variables|Default|GetPlayer))) true true "(R=0.930721,G=1.000000,B=0.100721,A=1.000000)")
      (if (Math|Boolean|ANDBoolean _returnvalue _returnvalue_2 (Utilities|IsValid (Variables|Default|GetPlayer)))
        (Class|BattleManager|Initialize (Variables|Default|GetBattleManager) (Variables|Default|GetPlayer) (Variables|Default|GetBoss) 0)
        (Class|BattleManager|StartBattle (Variables|Default|GetBattleManager))
        (else
          (Development|PrintString "Error"))))
    (:CastFailed
      (Development|PrintString "cast failed"))))

(event EventBeginPlay)

(event EventTick
  (params (DeltaSeconds :type Float%20%28single-precision%29)))

(fn ConstructionScript)

(fn AutoFind
  (if (Utilities|IsValid (Variables|Default|GetBattleManager))
    _
    (else
      (bind _outactors (Actor|GetAllActorsOfClass "/Script/CatheralBattle.BattleManager"))
      (Variables|Default|SetBattleManager (Utilities|Array|Get(acopy) _outactors))))
  (bind _outactors_2 (Actor|GetAllActorsOfClass "/Script/CatheralBattle.Boss_Sevarog"))
  (Variables|Default|SetBoss (Utilities|Array|Get(acopy) _outactors_2)))