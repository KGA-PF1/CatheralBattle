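; Playable boss character Blueprint that maps keyboard and mouse input to sprinting, skills, guard and melee attacks, mostly using GreyStone montages.
; Q, E, R and right-click play montages through DoOnce gates, and run input switches walk speed.
; Left-click drives a looping three-hit combo, with ComboAttackSave continuing buffered attacks and ResetCombo clearing state.
; The R ultimate temporarily snaps the camera boom to a mesh socket and disables movement.
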(event Custom|ResetCombo
  ;[1 1 1] 콤보 어택 관련
  ;;[0.9673 1 0.2732] 카운트 0번으로 다시 회귀후 변수 False 값으로 재설정
  (Variables|Default|SetAttackCount 0)
  (Variables|Default|SetSaveAttack false)
  (Variables|Default|SetIsAttacking false))

(event Custom|ComboAttackSave
  (bind _meleespeed (Variables|Default|GetMeleeSpeed))
  ;[1 1 1] 콤보 어택 관련
  (if (Variables|Default|GetSaveAttack)
    (Variables|Default|SetSaveAttack false)
    ;;[0.5943 0 1] 0에서 1번, 1에서 2번, 2에서 0번
    ;; 0에서 1번, 1에서 2번, 2에서 0번
    ;; ...무한 반복
    (switch int (Variables|Default|GetAttackCount)
      (:0
        ;;[0 1 0.9862] Attack Count 1 몽타주
        (Variables|Default|SetAttackCount 1)
        (Animation|PlayAnimMontage "/Game/TeamShare/TeamShare_CSW/Player/Montage/GreyStone_Attack_A.GreyStone_Attack_A" _meleespeed "None"))
      (:1
        ;;[0 1 0.9705] Attack Count 2 몽타주
        (Variables|Default|SetAttackCount 2)
        (Animation|PlayAnimMontage "/Game/TeamShare/TeamShare_CSW/Player/Montage/GreyStone_Attack_B.GreyStone_Attack_B" _meleespeed "None"))
      (:2
        ;;[0 1 0.9629] Attack Count 0 몽타주
        (Variables|Default|SetAttackCount 0)
        (Animation|PlayAnimMontage "/Game/TeamShare/TeamShare_CSW/Player/Montage/GreyStone_Attack_C.GreyStone_Attack_C" _meleespeed "None")))))

(event EventBeginPlay)

(event Input|ActionEvents|InputActionInputAction_Run
  (params (Key :type Key%20Structure :default "None"))
  ;[1 1 1] 달리기
  (:Pressed
    (Variables|/Script/Engine.CharacterMovementComponent|SetMaxWalkSpeed (Variables|Character|GetCharacterMovement) 6e+02))
  (:Released
    (Variables|/Script/Engine.CharacterMovementComponent|SetMaxWalkSpeed (Variables|Character|GetCharacterMovement) 4e+02)))

(event Input|MouseEvents|LeftMouseButton
  (params (Key :type Key%20Structure :default "None"))
  (:Pressed
    ;[1 1 1] 근접 공격 속도
    (Variables|Default|SetMeleeSpeed 1.2)
    ;[1 1 1] 콤보 어택 관련
    (if (Variables|Default|GetIsAttacking)
      (Variables|Default|SetSaveAttack true)
      (else
        (Variables|Default|SetIsAttacking true)
        ;;[0.5943 0 1] 0에서 1번, 1에서 2번, 2에서 0번
        ;; 0에서 1번, 1에서 2번, 2에서 0번
        ;; ...무한 반복
        (switch int (Variables|Default|GetAttackCount)
          (:0
            ;;[0 1 0.9862] Attack Count 1 몽타주
            (Variables|Default|SetAttackCount 1)
            (Animation|PlayAnimMontage "/Game/TeamShare/TeamShare_CSW/Player/Montage/GreyStone_Attack_A.GreyStone_Attack_A" (Variables|Default|GetMeleeSpeed) "None"))
          (:1
            ;;[0 1 0.9705] Attack Count 2 몽타주
            (Variables|Default|SetAttackCount 2)
            (Animation|PlayAnimMontage "/Game/TeamShare/TeamShare_CSW/Player/Montage/GreyStone_Attack_B.GreyStone_Attack_B" (Variables|Default|GetMeleeSpeed) "None"))
          (:2
            ;;[0 1 0.9629] Attack Count 0 몽타주
            (Variables|Default|SetAttackCount 0)
            (Animation|PlayAnimMontage "/Game/TeamShare/TeamShare_CSW/Player/Montage/GreyStone_Attack_C.GreyStone_Attack_C" (Variables|Default|GetMeleeSpeed) "None")))))))

(event Input|KeyboardEvents|R
  (params (Key :type Key%20Structure :default "None"))
  ;[1 1 1] 궁극기 (R)
  (:Pressed
    (Utilities|FlowControl|DoOnce false :!label _label
      (:Completed
        (Animation|PlayAnimMontage "/Game/TeamShare/TeamShare_CSW/Player/Montage/GreyStone_Ultimate.GreyStone_Ultimate" 1.0 "None")
        (Transformation|AttachComponentToComponent (Variables|Default|GetCameraBoom) (Variables|Character|GetMesh) "HoverAttachPoint" "SnapToTarget" "KeepRelative" "KeepRelative" true)
        (Pawn|Components|CharacterMovement|DisableMovement (Variables|Character|GetCharacterMovement))
        (Utilities|FlowControl|Delay 4.0)
        (Transformation|AttachComponentToComponent (Variables|Default|GetCameraBoom) (Variables|Default|GetCapsuleComponent) "None" "KeepRelative" "KeepRelative" "KeepRelative" false)
        (Pawn|Components|CharacterMovement|SetMovementMode (Variables|Character|GetCharacterMovement) "MOVE_Walking" 0)
        (goto _label Reset)))))

(event Input|KeyboardEvents|E
  (params (Key :type Key%20Structure :default "None"))
  ;[1 1 1] E 스킬
  (:Pressed
    (Utilities|FlowControl|DoOnce false :!label _label
      (:Completed
        (Animation|PlayAnimMontage "/Game/TeamShare/TeamShare_CSW/Player/Montage/GreyStone_Skill_B.GreyStone_Skill_B" 1.0 "None")
        (Utilities|FlowControl|Delay 1.0)
        (goto _label Reset)))))

(event Input|KeyboardEvents|Q
  (params (Key :type Key%20Structure :default "None"))
  (:Pressed
    (Utilities|FlowControl|DoOnce false :!label _label
      (:Completed
        (Animation|PlayAnimMontage "/Game/TeamShare/TeamShare_CSW/Boss/Montage/Boss_Skill1.Boss_Skill1" 1.0 "None")
        (goto _label Reset)))))

(event Input|MouseEvents|RightMouseButton
  (params (Key :type Key%20Structure :default "None"))
  ;[1 1 1] 방어
  (:Pressed
    (Utilities|FlowControl|DoOnce false :!label _label
      (:Completed
        (Animation|PlayAnimMontage "/Game/TeamShare/TeamShare_CSW/Player/Montage/GreyStone_Guard.GreyStone_Guard" 1.0 "None")
        (Utilities|FlowControl|Delay 1.0)
        (goto _label Reset)))))

(fn ConstructionScript)