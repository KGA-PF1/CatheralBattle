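; Player character with Greystone melee combat: a three-hit left-click combo, right-click guard, two skills, an ultimate and a run toggle held by input.
; The combo buffers clicks made mid-attack; ComboAttackSave chains the next montage and ResetCombo clears the state.
; Skills and guard use DoOnce gates reset after delays, with Q launching upward and R temporarily attaching the camera boom to a mesh socket while movement is disabled.
; Input starts disabled briefly on BeginPlay.
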(event Custom|ResetCombo
  ;[1 1 1] Combo System Setup.
  (Variables|Default|SetAttackCount 0)
  (Variables|Default|SetSaveAttack false)
  (Variables|Default|SetIsAttacking false))

(event Custom|ComboAttackSave
  (bind _meleespeed (Variables|Default|GetMeleeSpeed))
  ;[1 1 1] Combo System Setup.
  (if (Variables|Default|GetSaveAttack)
    (Variables|Default|SetSaveAttack false)
    (switch int (Variables|Default|GetAttackCount)
      (:0
        (Variables|Default|SetAttackCount 1)
        (Animation|PlayAnimMontage "/Game/TeamShare/TeamShare_CSW/Montage/GreyStone_Attack_A.GreyStone_Attack_A" _meleespeed "None"))
      (:1
        (Variables|Default|SetAttackCount 2)
        (Animation|PlayAnimMontage "/Game/TeamShare/TeamShare_CSW/Montage/GreyStone_Attack_B.GreyStone_Attack_B" _meleespeed "None"))
      (:2
        (Variables|Default|SetAttackCount 0)
        (Animation|PlayAnimMontage "/Game/TeamShare/TeamShare_CSW/Montage/GreyStone_Attack_C.GreyStone_Attack_C" _meleespeed "None")))))

(event EventBeginPlay
  (Input|DisableInput 0)
  (Utilities|FlowControl|Delay 5.0)
  (Input|EnableInput 0))

(event Input|ActionEvents|InputActionInputAction_Run
  (params (Key :type Key%20Structure :default "None"))
  (:Pressed
    (Variables|/Script/Engine.CharacterMovementComponent|SetMaxWalkSpeed (Variables|Character|GetCharacterMovement) 6e+02))
  (:Released
    (Variables|/Script/Engine.CharacterMovementComponent|SetMaxWalkSpeed (Variables|Character|GetCharacterMovement) 4e+02)))

(event Input|MouseEvents|LeftMouseButton
  (params (Key :type Key%20Structure :default "None"))
  ;[1 1 1] Simple attack setup. Intentionally not using inputs so that this will "just work" with the 3rd Person Template. If you were doing this for real, you would set up a proper input.
  (:Pressed
    (Variables|Default|SetMeleeSpeed 1.2)
    ;[1 1 1] Combo System Setup.
    (if (Variables|Default|GetIsAttacking)
      (Variables|Default|SetSaveAttack true)
      (else
        (Variables|Default|SetIsAttacking true)
        (switch int (Variables|Default|GetAttackCount)
          (:0
            (Variables|Default|SetAttackCount 1)
            (Animation|PlayAnimMontage "/Game/TeamShare/TeamShare_CSW/Montage/GreyStone_Attack_A.GreyStone_Attack_A" (Variables|Default|GetMeleeSpeed) "None"))
          (:1
            (Variables|Default|SetAttackCount 2)
            (Animation|PlayAnimMontage "/Game/TeamShare/TeamShare_CSW/Montage/GreyStone_Attack_B.GreyStone_Attack_B" (Variables|Default|GetMeleeSpeed) "None"))
          (:2
            (Variables|Default|SetAttackCount 0)
            (Animation|PlayAnimMontage "/Game/TeamShare/TeamShare_CSW/Montage/GreyStone_Attack_C.GreyStone_Attack_C" (Variables|Default|GetMeleeSpeed) "None")))))))

(event Input|KeyboardEvents|R
  (params (Key :type Key%20Structure :default "None"))
  (:Pressed
    (Utilities|FlowControl|DoOnce false :!label _label
      (:Completed
        (Animation|PlayAnimMontage "/Game/TeamShare/TeamShare_CSW/Montage/GreyStone_Ultimate.GreyStone_Ultimate" 1.0 "None")
        (Transformation|AttachComponentToComponent (Variables|Default|GetCameraBoom) (Variables|Character|GetMesh) "HoverAttachPoint" "SnapToTarget" "KeepRelative" "KeepRelative" true)
        (Pawn|Components|CharacterMovement|DisableMovement (Variables|Character|GetCharacterMovement))
        (Utilities|FlowControl|Delay 4.0)
        (Transformation|AttachComponentToComponent (Variables|Default|GetCameraBoom) (Variables|Default|GetCapsuleComponent) "None" "KeepRelative" "KeepRelative" "KeepRelative" false)
        (Pawn|Components|CharacterMovement|SetMovementMode (Variables|Character|GetCharacterMovement) "MOVE_Walking" 0)
        (goto _label Reset)))))

(event Input|KeyboardEvents|E
  (params (Key :type Key%20Structure :default "None"))
  (:Pressed
    (Utilities|FlowControl|DoOnce false :!label _label
      (:Completed
        (Animation|PlayAnimMontage "/Game/TeamShare/TeamShare_CSW/Montage/GreyStone_Skill_B.GreyStone_Skill_B" 1.0 "None")
        (Utilities|FlowControl|Delay 1.0)
        (goto _label Reset)))))

(event Input|KeyboardEvents|Q
  (params (Key :type Key%20Structure :default "None"))
  (:Pressed
    (Utilities|FlowControl|DoOnce false :!label _label
      (:Completed
        (Character|Jump)
        (Character|LaunchCharacter "0.000000,0.000000,700.000000" false false)
        (Animation|PlayAnimMontage "/Game/TeamShare/TeamShare_CSW/Montage/GreyStone_Skill_A.GreyStone_Skill_A" 1.0 "None")
        (Utilities|FlowControl|Delay 1.0)
        (Pawn|Components|CharacterMovement|DisableMovement (Variables|Character|GetCharacterMovement))
        (Utilities|FlowControl|Delay 1.0)
        (Pawn|Components|CharacterMovement|SetMovementMode (Variables|Character|GetCharacterMovement) "MOVE_Walking" 0)
        (goto _label Reset)))))

(event Input|MouseEvents|RightMouseButton
  (params (Key :type Key%20Structure :default "None"))
  (:Pressed
    (Utilities|FlowControl|DoOnce false :!label _label
      (:Completed
        (Animation|PlayAnimMontage "/Game/TeamShare/TeamShare_CSW/Montage/GreyStone_Guard.GreyStone_Guard" 1.0 "None")
        (Utilities|FlowControl|Delay 1.0)
        (goto _label Reset)))))

(fn ConstructionScript)