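; BP_Monster is a monster actor with test logic for attacking and damaging the player.
; On BeginPlay it casts the first player pawn to BP_PlayerCharacter and caches the reference.
; Pressing K calls PerformAttack and applies fixed damage directly to the cached player, with no range or hit check in this graph.
; Every Tick it prints the player's current HP as debug output.
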(event EventBeginPlay
  (bind _asbp_player_character (Utilities|Casting|CastToBP_PlayerCharacter (Game|Player|GetPlayerPawn 0)))
  (Variables|Default|SetPlayer _asbp_player_character))

(event Collision|EventActorBeginOverlap
  (params (OtherActor :type Actor%20Object%20Reference)))

(event EventTick
  (params (DeltaSeconds :type Float%20%28single-precision%29))
  (bind _returnvalue (Class|PlayerCharacter|GetHp (Variables|Default|GetPlayer)))
  (Development|PrintString (Utilities|String|ToString(Float) _returnvalue)))

(event Input|KeyboardEvents|K
  (params (Key :type Key%20Structure :default "None"))
  (:Pressed
    (Class|Monster|PerformAttack)
    (Class|PlayerCharacter|TakeDamage (Variables|Default|GetPlayer) 1e+01)))

(fn ConstructionScript)