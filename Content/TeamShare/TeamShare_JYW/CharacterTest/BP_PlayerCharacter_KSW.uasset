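; Player character Blueprint that implements a looping three-hit GreyStone melee combo.
; The Enhanced Input attack action, gated by CanAttack, starts the combo or buffers the press in SaveAttack while an attack is active.
; AttackCount cycles through montages A, B and C at a slightly raised play rate.
; ComboAttackSave consumes a buffered press to play the next montage, and ResetCombo clears the count and flags.
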(event Custom|ResetCombo
  ;[1 1 1] 콤보 어택 관련
  ;;[0.9673 1 0.2732] 카운트 0번으로 다시 회귀후 변수 False 값으로 재설정
  (Variables|Default|SetAttackCount 0)
  (Variables|Default|SetSaveAttack false)
  (Variables|Default|SetIsAttacking false))

(event Custom|ComboAttackSave
  (bind _meleespeed (Variables|Default|GetMeleeSpeed))
  ;[1 1 1] 콤보 어택 관련
  (if (Variables|Default|GetSaveAttack)
    (Variables|Default|SetSaveAttack false)
    ;;[0.5943 0 1] 0에서 1번, 1에서 2번, 2에서 0번
    ;; 0에서 1번, 1에서 2번, 2에서 0번
    ;; ...무한 반복
    (switch int (Variables|Default|GetAttackCount)
      (:0
        ;;[0 1 0.9862] Attack Count 1 몽타주
        (Variables|Default|SetAttackCount 1)
        (Animation|PlayAnimMontage "/Game/TeamShare/TeamShare_CSW/Player/Montage/GreyStone_Attack_A.GreyStone_Attack_A" _meleespeed "None"))
      (:1
        ;;[0 1 0.9705] Attack Count 2 몽타주
        (Variables|Default|SetAttackCount 2)
        (Animation|PlayAnimMontage "/Game/TeamShare/TeamShare_CSW/Player/Montage/GreyStone_Attack_B.GreyStone_Attack_B" _meleespeed "None"))
      (:2
        ;;[0 1 0.9629] Attack Count 0 몽타주
        (Variables|Default|SetAttackCount 0)
        (Animation|PlayAnimMontage "/Game/TeamShare/TeamShare_CSW/Player/Montage/GreyStone_Attack_C.GreyStone_Attack_C" _meleespeed "None")))))

(event Input|EnhancedActionEvents|EnhancedInputActionIA_Attack
  (params (ActionValue :type Boolean) (ElapsedSeconds :type Float%20%28double-precision%29) (TriggeredSeconds :type Float%20%28double-precision%29) (InputAction :type Input%20Action%20Object%20Reference :default "/Game/TeamShare/TeamShare_JYW/Input/IA_Attack.IA_Attack"))
  (:Started
    (if (Variables|Default|GetbCanAttack)
      ;[1 1 1] 근접 공격 속도
      (Variables|Default|SetMeleeSpeed 1.2)
      ;[1 1 1] 콤보 어택 관련
      (if (Variables|Default|GetIsAttacking)
        (Variables|Default|SetSaveAttack true)
        (else
          (Variables|Default|SetIsAttacking true)
          ;;[0.5943 0 1] 0에서 1번, 1에서 2번, 2에서 0번
          ;; 0에서 1번, 1에서 2번, 2에서 0번
          ;; ...무한 반복
          (switch int (Variables|Default|GetAttackCount)
            (:0
              ;;[0 1 0.9862] Attack Count 1 몽타주
              (Variables|Default|SetAttackCount 1)
              (Animation|PlayAnimMontage "/Game/TeamShare/TeamShare_CSW/Player/Montage/GreyStone_Attack_A.GreyStone_Attack_A" (Variables|Default|GetMeleeSpeed) "None"))
            (:1
              ;;[0 1 0.9705] Attack Count 2 몽타주
              (Variables|Default|SetAttackCount 2)
              (Animation|PlayAnimMontage "/Game/TeamShare/TeamShare_CSW/Player/Montage/GreyStone_Attack_B.GreyStone_Attack_B" (Variables|Default|GetMeleeSpeed) "None"))
            (:2
              ;;[0 1 0.9629] Attack Count 0 몽타주
              (Variables|Default|SetAttackCount 0)
              (Animation|PlayAnimMontage "/Game/TeamShare/TeamShare_CSW/Player/Montage/GreyStone_Attack_C.GreyStone_Attack_C" (Variables|Default|GetMeleeSpeed) "None"))))))))

(event EventBeginPlay)

(event Collision|EventActorBeginOverlap
  (params (OtherActor :type Actor%20Object%20Reference)))

(event EventTick
  (params (DeltaSeconds :type Float%20%28single-precision%29)))

(event Input|MouseEvents|LeftMouseButton
  (params (Key :type Key%20Structure)))

(fn ConstructionScript)